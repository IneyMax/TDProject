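; BP_Bullet_Base is a bullet projectile actor that flies forward and damages what it hits.
; Tick moves it along its forward vector at BulletSpeed with a swept offset, with no projectile movement node, and destroys it on a blocking hit.
; The Sphere component's hit event sends a fixed TakeDamageMessage to the other actor, then destroys the bullet.
; A delay from BeginPlay caps its lifetime at one second.
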(event OnComponentHit(Sphere)
  (params (HitComponent :type Primitive%20Component%20Object%20Reference) (OtherActor :type Actor%20Object%20Reference) (OtherComp :type Primitive%20Component%20Object%20Reference) (NormalImpulse :type Vector :default "0, 0, 0") (Hit :type Hit%20Result%20Structure%20%28by%20ref%29))
  (Class|BPITakingDamage|TakeDamage(Message) OtherActor 1e+01)
  (Actor|DestroyActor))

(event EventTick
  (params (DeltaSeconds :type Float%20%28single-precision%29))
  (bind _sweephitresult (Transformation|AddActorWorldOffset (* (Transformation|GetActorForwardVector) (* DeltaSeconds (Variables|Default|GetBulletSpeed))) true))
  (if (.bBlockingHit (Collision|BreakHitResult _sweephitresult))
    (Actor|DestroyActor)))

(event EventBeginPlay
  (Utilities|FlowControl|Delay 1.0)
  (Actor|DestroyActor))

(fn ConstructionScript)