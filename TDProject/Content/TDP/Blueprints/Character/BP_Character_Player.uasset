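; BP_Character_Player is the player character Blueprint, handling input for shooting, weapon switching and amplifier use.
; Two select inputs set the active weapon index, then refresh BPWeaponComponent with the matching weapon and ammo items from InventoryComponent slots.
; The fire input starts and ends shooting on the weapon component, while the amplifier input messages the active index's amplifier item, passing the character.
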(event Input|ActionEvents|InputActionSelectActiveSlot_1
  (params (Key :type Key%20Structure :default "None"))
  (:Pressed
    (if (!= (Variables|Default|GetIndexActiveWeapon) (Variables|Default|GetIndexActiveSlot_1))
      (Variables|Default|SetIndexActiveWeapon 0)
      (Default|RefreshWeapon (Variables|Default|GetBP_Weapon_Component) (Class|TDInventoryComponent|GetSlottedItem (Variables|Default|GetInventoryComponent) (Utilities|Array|Get(acopy) (Variables|Default|GetAmmoSlots) (Variables|Default|GetIndexActiveWeapon))) (Class|TDInventoryComponent|GetSlottedItem (Variables|Default|GetInventoryComponent) (Utilities|Array|Get(acopy) (Variables|Default|GetWeaponSlots) (Variables|Default|GetIndexActiveWeapon)))))))

(event Input|ActionEvents|InputActionSelectActiveSlot_2
  (params (Key :type Key%20Structure :default "None"))
  (:Pressed
    (if (!= (Variables|Default|GetIndexActiveWeapon) (Variables|Default|GetIndexActiveSlot_2))
      (Variables|Default|SetIndexActiveWeapon 1)
      (Default|RefreshWeapon (Variables|Default|GetBP_Weapon_Component) (Class|TDInventoryComponent|GetSlottedItem (Variables|Default|GetInventoryComponent) (Utilities|Array|Get(acopy) (Variables|Default|GetAmmoSlots) (Variables|Default|GetIndexActiveWeapon))) (Class|TDInventoryComponent|GetSlottedItem (Variables|Default|GetInventoryComponent) (Utilities|Array|Get(acopy) (Variables|Default|GetWeaponSlots) (Variables|Default|GetIndexActiveWeapon)))))))

(event Input|ActionEvents|InputActionUseActiveSlot
  (params (Key :type Key%20Structure :default "None"))
  (bind _bp_weapon_component (Variables|Default|GetBP_Weapon_Component))
  (:Pressed
    (Default|StartShoot _bp_weapon_component))
  (:Released
    (Default|EndShoot _bp_weapon_component)))

(event Input|ActionEvents|InputActionUseAmplifier
  (params (Key :type Key%20Structure :default "None"))
  (:Pressed
    (Class|BPIAmplifier|UseAmplifier(Message) (Class|TDInventoryComponent|GetSlottedItem (Variables|Default|GetInventoryComponent) (Utilities|Array|Get(acopy) (Variables|Default|GetAmplifierSlots) (Variables|Default|GetIndexActiveWeapon))) self)))

(fn ConstructionScript
  (|CallParentFunction))