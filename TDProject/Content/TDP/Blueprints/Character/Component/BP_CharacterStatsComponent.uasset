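; Character stats component that tracks a character's health through damage and recovery.
; TakeDamage subtracts from CurrentHP, then fires damage and health-change dispatchers while HP stays above zero, or only the health-is-over dispatcher otherwise.
; RecoverHealth adds to CurrentHP without clamping to MaxHP or broadcasting a health change.
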(event Custom|RecoverHealth
  (params (Health :type Float%20%28single-precision%29))
  (Variables|Default|SetCurrent%20HP (+ Health (Variables|Default|GetCurrent%20HP))))

(event Custom|TakeDamage
  (params (Damage :type Float%20%28single-precision%29) (DamageSource :type Actor%20Object%20Reference))
  (bind _output_get (Variables|Default|SetCurrent%20HP (- (Variables|Default|GetCurrent%20HP) Damage)))
  (if (> _output_get 0.0)
    (Default|CallOnTakeDamage Damage DamageSource)
    (Default|CallOnChangeHealth (Variables|Default|GetCurrent%20HP) (Variables|Default|GetMax%20HP))
    (else
      (Default|CallOnHealthIsOver))))